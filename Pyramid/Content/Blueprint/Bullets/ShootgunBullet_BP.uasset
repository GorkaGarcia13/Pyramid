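; Shotgun projectile Blueprint that damages and knocks back enemies on overlap and has a short lifetime.
; Any overlap on BulletColl spawns a scaled-down explosion effect and sound, but only BaseEnemy hits continue.
; Those enemies have their capsule shifted along the bullet's velocity by Retention, without sweep, and take BulletDamage before the bullet destroys itself.
; Root component activation starts a brief delay that also destroys the bullet.
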(event `self.BulletColl.OnComponentBeginOverlap`
  (params (OverlappedComponent :type "PrimitiveComponent Object Reference") (OtherActor :type "Actor Object Reference") (OtherComp :type "PrimitiveComponent Object Reference") (OtherBodyIndex :type Integer) (bFromSweep :type Boolean) (SweepResult :type "HitResult Structure (by ref)"))
  (bind _returnvalue (`self.K2_GetActorLocation` self))
  ;[1 1 1] BulletHit
  (`GameplayStatics.SpawnEmitterAtLocation` "/Game/StarterContent/Particles/P_Explosion.P_Explosion" _returnvalue (struct) (0.5 0.5 0.5) false)
  (`GameplayStatics.PlaySoundAtLocation` "/Game/StarterContent/Audio/Explosion_Cue.Explosion_Cue" _returnvalue)
  (bind _asbase_enemy (cast `/Game/Enemies/BaseEnemy` OtherActor))
  (bind _capsulecomponent (`Character.CapsuleComponent` _asbase_enemy))
  (`SceneComponent.K2_SetWorldLocation` _capsulecomponent (+ (`SceneComponent.K2_GetComponentLocation` _capsulecomponent) (* (`KismetMathLibrary.Normal` (`self.GetVelocity`)) (`self.Retention`))) false false)
  (`/Game/Blueprint/Components/HealthComponent.ReceiveDamage` (`/Game/Enemies/BaseEnemy.HealthComponent` _asbase_enemy) (`self.BulletDamage`))
  (`self.K2_DestroyActor`))

(event `self.DefaultSceneRoot.OnComponentActivated`
  (params (Component :type "ActorComponent Object Reference") (bReset :type Boolean))
  (`KismetSystemLibrary.Delay` 0.3)
  (`self.K2_DestroyActor` self))

(fn `UserConstructionScript`
  (`parent.UserConstructionScript`))
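; Revolver weapon Blueprint that fires RifleBullet_BP projectiles from its FireDirection component, with primary and secondary modes.
; Each trigger event fires at once, then repeats through a looping timer by function name at that mode's fire rate.
; Primary spawns one bullet per shot; secondary waits on a Delay, then spawns a burst of enlarged bullets in one loop.
; Releasing the trigger clears both timers and resets the shooting flags.
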(event `PullTrigger`
  ;[1 1 1] ShootLoop
  (`self.PrincipalShoot`)
  (`KismetSystemLibrary.K2_SetTimer` null "PrincipalShoot" (`self.FireRatePrincipal`) true))

(event `PullSpecialTrigger`
  ;[1 1 1] ShootLoop
  (`self.SecondaryShoot`)
  (`KismetSystemLibrary.K2_SetTimer` null "SecondaryShoot" (`self.FireRateSecondary`) true))

(event `ReleaseTrigger`
  ;[1 1 1] ShootLoop
  (`KismetSystemLibrary.K2_ClearTimer` null "PrincipalShoot")
  (`KismetSystemLibrary.K2_ClearTimer` null "SecondaryShoot")
  (set `self.IsShootingPrincipal?` false)
  (set `self.IsShootingSecondary?` false))

(event `SecondaryShoot`
  (`KismetSystemLibrary.Delay` 1.0)
  (for _ (range 7)
    (`|SpawnActorFromClass` "/Game/Blueprint/Bullets/RifleBullet_BP.RifleBullet_BP_C" (`KismetMathLibrary.MakeTransform` (.location (`SceneComponent.K2_GetComponentToWorld` (`self.FireDirection`))) (.rotation (`SceneComponent.K2_GetComponentToWorld` (`self.FireDirection`))) (3.0 3.0 3.0)) "AdjustIfPossibleButDontSpawnIfColliding" "OverrideRootScale" null (`self.GetInstigator`))))

(event `PrincipalShoot`
  (`|SpawnActorFromClass` "/Game/Blueprint/Bullets/RifleBullet_BP.RifleBullet_BP_C" (`SceneComponent.K2_GetComponentToWorld` (`self.FireDirection`)) "AdjustIfPossibleButDontSpawnIfColliding" "OverrideRootScale" null (`self.GetInstigator`)))

(fn `UserConstructionScript`
  (`parent.UserConstructionScript`))
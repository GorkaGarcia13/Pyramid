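; Shotgun weapon that fires bursts of ShootgunBullet_BP pellets in primary and secondary modes.
; Each trigger pull fires immediately, then repeats on a looping timer at that mode's fire rate until ReleaseTrigger clears both timers.
; Pellets spawn at random points inside box components, with random pitch and yaw spread around paired direction components.
; Primary fire uses one box and direction pair, while secondary fire uses three, tripling the pellets.
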(event `PullTrigger`
  ;[1 1 1] ShootLoop
  (`self.PrincipalShoot`)
  (`KismetSystemLibrary.K2_SetTimer` null "PrincipalShoot" (`self.FireRatePrincipal`) true))

(event `PullSpecialTrigger`
  ;[1 1 1] ShootLoop
  (`self.SecondaryShoot`)
  (`KismetSystemLibrary.K2_SetTimer` null "SecondaryShoot" (`self.FireRateSecondary`) true))

(event `ReleaseTrigger`
  ;[1 1 1] ShootLoop
  (`KismetSystemLibrary.K2_ClearTimer` null "PrincipalShoot")
  (`KismetSystemLibrary.K2_ClearTimer` null "SecondaryShoot")
  (set `self.IsShootingPrimary?` false)
  (set `self.IsShootingSecondary?` false))

(event `PrincipalShoot`
  (bind _dispersionbox (`self.DispersionBox`))
  (for _ (range 8)
    (`|SpawnActorFromClass` "/Game/Blueprint/Bullets/ShootgunBullet_BP.ShootgunBullet_BP_C" (`KismetMathLibrary.MakeTransform` (`KismetMathLibrary.RandomPointInBoundingBox` (`SceneComponent.K2_GetComponentLocation` _dispersionbox) (`BoxComponent.GetScaledBoxExtent` _dispersionbox)) (`KismetMathLibrary.MakeRotator` (.roll (`SceneComponent.K2_GetComponentRotation` (`self.FireDirection`))) (+ (.pitch (`SceneComponent.K2_GetComponentRotation` (`self.FireDirection`))) (`KismetMathLibrary.RandomFloatInRange` -5.0 5.0)) (+ (.yaw (`SceneComponent.K2_GetComponentRotation` (`self.FireDirection`))) (`KismetMathLibrary.RandomFloatInRange` -5.0 5.0))) (1.0 1.0 1.0)) "AdjustIfPossibleButDontSpawnIfColliding" "OverrideRootScale" null (`self.GetInstigator`))))

(event `SecondaryShoot`
  (bind _dispersionbox (`self.DispersionBox`))
  (bind _box (`self.Box`))
  (bind _box1 (`self.Box1`))
  (for _ (range 8)
    (`|SpawnActorFromClass` "/Game/Blueprint/Bullets/ShootgunBullet_BP.ShootgunBullet_BP_C" (`KismetMathLibrary.MakeTransform` (`KismetMathLibrary.RandomPointInBoundingBox` (`SceneComponent.K2_GetComponentLocation` _dispersionbox) (`BoxComponent.GetScaledBoxExtent` _dispersionbox)) (`KismetMathLibrary.MakeRotator` (.roll (`SceneComponent.K2_GetComponentRotation` (`self.FireDirection`))) (+ (.pitch (`SceneComponent.K2_GetComponentRotation` (`self.FireDirection`))) (`KismetMathLibrary.RandomFloatInRange` -5.0 5.0)) (+ (.yaw (`SceneComponent.K2_GetComponentRotation` (`self.FireDirection`))) (`KismetMathLibrary.RandomFloatInRange` -5.0 5.0)))) "AdjustIfPossibleButDontSpawnIfColliding" "OverrideRootScale" null (`self.GetInstigator`))
    (`|SpawnActorFromClass` "/Game/Blueprint/Bullets/ShootgunBullet_BP.ShootgunBullet_BP_C" (`KismetMathLibrary.MakeTransform` (`KismetMathLibrary.RandomPointInBoundingBox` (`SceneComponent.K2_GetComponentLocation` _box) (`BoxComponent.GetScaledBoxExtent` _box)) (`KismetMathLibrary.MakeRotator` (.roll (`SceneComponent.K2_GetComponentRotation` (`self.Arrow`))) (+ (.pitch (`SceneComponent.K2_GetComponentRotation` (`self.Arrow`))) (`KismetMathLibrary.RandomFloatInRange` -5.0 5.0)) (+ (.yaw (`SceneComponent.K2_GetComponentRotation` (`self.Arrow`))) (`KismetMathLibrary.RandomFloatInRange` -5.0 5.0)))) "AdjustIfPossibleButDontSpawnIfColliding" "OverrideRootScale" null (`self.GetInstigator`))
    (`|SpawnActorFromClass` "/Game/Blueprint/Bullets/ShootgunBullet_BP.ShootgunBullet_BP_C" (`KismetMathLibrary.MakeTransform` (`KismetMathLibrary.RandomPointInBoundingBox` (`SceneComponent.K2_GetComponentLocation` _box1) (`BoxComponent.GetScaledBoxExtent` _box1)) (`KismetMathLibrary.MakeRotator` (.roll (`SceneComponent.K2_GetComponentRotation` (`self.Arrow1`))) (+ (.pitch (`SceneComponent.K2_GetComponentRotation` (`self.Arrow1`))) (`KismetMathLibrary.RandomFloatInRange` -5.0 5.0)) (+ (.yaw (`SceneComponent.K2_GetComponentRotation` (`self.Arrow1`))) (`KismetMathLibrary.RandomFloatInRange` -5.0 5.0)))) "AdjustIfPossibleButDontSpawnIfColliding" "OverrideRootScale" null (`self.GetInstigator`))))

(fn `UserConstructionScript`
  (`parent.UserConstructionScript`))
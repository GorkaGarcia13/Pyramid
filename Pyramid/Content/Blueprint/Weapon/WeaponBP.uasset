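; Weapon Blueprint that fires bullets automatically while its trigger is held.
; PullTrigger spawns one projectile at once and starts a looping timer on SpawnProyectile at FireRate, which ReleaseTrigger clears.
; Each shot casts the instigator to Char_BP and spawns a Bullet at that character's BulletArrow transform, passing the instigator along.
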(event `PullTrigger`
  ;[1 1 1] ShootLoop
  (`self.SpawnProyectile`)
  (`KismetSystemLibrary.K2_SetTimer` null "SpawnProyectile" (`self.FireRate`) true))

(event `ReleaseTrigger`
  ;[1 1 1] ShootLoop
  (`KismetSystemLibrary.K2_ClearTimer` null "SpawnProyectile"))

(event `SpawnProyectile`
  (bind _returnvalue (`self.GetInstigator`))
  ;[1 1 1] SpawnProyectile
  (bind _aschar_bp (cast `/Game/Blueprint/Character/Char_BP` _returnvalue))
  (`|SpawnActorFromClass` "/Game/Blueprint/Bullets/Bullet.Bullet_C" (`SceneComponent.K2_GetComponentToWorld` (`/Game/Blueprint/Character/Char_BP.BulletArrow` _aschar_bp)) "Undefined" "OverrideRootScale" null _returnvalue))

(fn `UserConstructionScript`)
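; Rifle weapon Blueprint with a burst primary fire and an automatic secondary fire, both spawning RifleBullet_BP at the FireDirection transform.
; Pulling either trigger fires immediately, then repeats on a looping timer at that mode's fire rate.
; Primary fire chains three delayed shots behind an IsShootingPrincipal guard, while secondary fire spawns one bullet per tick of its timer.
; ReleaseTrigger clears both timers and resets the shooting flags.
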(event `PullTrigger`
  ;[1 1 1] ShootLoop
  (`self.PrincipalShoot`)
  (`KismetSystemLibrary.K2_SetTimer` null "PrincipalShoot" (`self.FireRatePrincipal`) true))

(event `PullSpecialTrigger`
  ;[1 1 1] ShootLoop
  (`self.SecondaryShoot`)
  (`KismetSystemLibrary.K2_SetTimer` null "SecondaryShoot" (`self.FireRateSecondary`) true))

(event `ReleaseTrigger`
  ;[1 1 1] ShootLoop
  (`KismetSystemLibrary.K2_ClearTimer` null "PrincipalShoot")
  (`KismetSystemLibrary.K2_ClearTimer` null "SecondaryShoot")
  (set `self.IsShootingPrincipal?` false)
  (set `self.IsShootingSecondary?` false))

(event `PrincipalShoot`
  ;[1 1 1] PrincipalShoot
  (if (not (`self.IsShootingPrincipal?`))
    (set `self.IsShootingPrincipal?` true)
    (`self.ShootBurst`)
    (`KismetSystemLibrary.Delay` 0.1)
    (`self.ShootBurst`)
    (`KismetSystemLibrary.Delay` 0.1)
    (`self.ShootBurst`)
    (`KismetSystemLibrary.Delay` 0.1)
    (set `self.IsShootingPrincipal?` false)))

(event `ShootBurst`
  ;[1 1 1] PrincipalShoot
  (`|SpawnActorFromClass` "/Game/Blueprint/Bullets/RifleBullet_BP.RifleBullet_BP_C" (`SceneComponent.K2_GetComponentToWorld` (`self.FireDirection`)) "AdjustIfPossibleButDontSpawnIfColliding" "OverrideRootScale" null (`self.GetInstigator`)))

(event `SecondaryShoot`
  ;[1 1 1] SecondaryShoot
  (`self.ShootAutomatic`))

(event `ShootAutomatic`
  ;[1 1 1] SecondaryShoot
  (`|SpawnActorFromClass` "/Game/Blueprint/Bullets/RifleBullet_BP.RifleBullet_BP_C" (`SceneComponent.K2_GetComponentToWorld` (`self.FireDirection`)) "AdjustIfPossibleButDontSpawnIfColliding" "OverrideRootScale" null (`self.GetInstigator`)))

(fn `UserConstructionScript`
  (`parent.UserConstructionScript`))
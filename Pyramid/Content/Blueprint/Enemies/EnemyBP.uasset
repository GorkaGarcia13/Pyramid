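; Enemy Blueprint that displays its maximum health as in-world text.
; On BeginPlay it calls the parent, then writes the HealthComponent's MaxHealth to a TextRender component.
; The text is set only at startup, with no update in this graph when health changes.
; Overlap and Tick events are disabled, and the construction script only calls its parent.
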(event `self.ReceiveBeginPlay`
  (`parent.ReceiveBeginPlay`)
  (`TextRenderComponent.K2_SetText` (`self.TextRender`) (`KismetTextLibrary.Conv_DoubleToText` (`/Game/Blueprint/Components/HealthComponent.MaxHealth` (`self.HealthComponent`)) "HalfToEven")))

(fn `UserConstructionScript`
  (`parent.UserConstructionScript`))
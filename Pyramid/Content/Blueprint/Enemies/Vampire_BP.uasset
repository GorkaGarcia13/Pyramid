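; Vampire enemy Blueprint that removes itself from the world once its health runs out.
; BeginPlay calls the parent, then starts a looping 0.2-second timer that runs the Dead event.
; Dead polls the HealthComponent and destroys the actor when current health is zero or below, using neither Tick nor a death notification.
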(event `self.ReceiveBeginPlay`
  (`parent.ReceiveBeginPlay`)
  (`KismetSystemLibrary.K2_SetTimer` null "Dead" 0.2 true))

(event `Dead`
  (if (<= (`/Game/Blueprint/Components/HealthComponent.CurrentHealth` (`self.HealthComponent`)) 0.0)
    (`self.K2_DestroyActor`)))

(fn `UserConstructionScript`
  (`parent.UserConstructionScript`))
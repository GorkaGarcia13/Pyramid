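; HealthComponent is a Blueprint component that tracks health and death state.
; On BeginPlay it sets current health to the maximum.
; ReceiveDamage subtracts the given amount while IsDead is false and sets that flag once health reaches zero or below, with no clamping or death notification.
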(event `self.ReceiveBeginPlay`
  ;[1 1 1] BeginPlay
  (set `self.CurrentHealth` (`self.MaxHealth`)))

(fn `ReceiveDamage`
  (params (Delta :type "Float (double-precision)"))
  ;[1 1 1] ReceiveDamage
  (if (not (`self.IsDead`))
    (bind _output_get (set `self.CurrentHealth` (- (`self.CurrentHealth`) Delta)))
    (if (<= _output_get 0.0)
      (set `self.IsDead` true))))
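; SpawnEnemy is a spawner actor that keeps adding Vampire_BP enemies to the level up to a limit.
; On BeginPlay it starts a looping two-second timer that calls its SpawnEnemy event.
; Each tick of the timer counts all Vampire_BP actors in the world and, while below MaxVampireEnemies, spawns one with SpawnAIFromClass at a random point inside the BoxColl volume.
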(event `self.ReceiveBeginPlay`
  (`KismetSystemLibrary.K2_SetTimer` null "SpawnEnemy" 2.0 true))

(event `SpawnEnemy`
  (bind _boxcoll (`self.BoxColl`))
  (bind _outactors (`GameplayStatics.GetAllActorsOfClass` "/Game/Blueprint/Enemies/Vampire_BP.Vampire_BP_C"))
  (if (<= (`KismetArrayLibrary.Array_Length` _outactors) (- (`self.MaxVampireEnemies`) 1))
    (`AIBlueprintHelperLibrary.SpawnAIFromClass` "/Game/Blueprint/Enemies/Vampire_BP.Vampire_BP_C" null (`KismetMathLibrary.RandomPointInBoundingBox` (`SceneComponent.K2_GetComponentLocation` _boxcoll) (`BoxComponent.GetScaledBoxExtent` _boxcoll)))))

(fn `UserConstructionScript`)
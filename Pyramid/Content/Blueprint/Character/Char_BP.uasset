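; Player character Blueprint that moves along world axes and carries a weapon.
; On BeginPlay it spawns a WeaponBP, stores it and snaps it to the mesh's right-hand socket.
; Fire input forwards press and release to the weapon's trigger functions.
; Look input is incomplete: Look_Up alone sets control rotation, feeding its value into both X and Y, while Look_Right does nothing.
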(event `self.ReceiveBeginPlay`
  ;[1 1 1] BeginPlay
  (bind _returnvalue (`|SpawnActorFromClass` "/Game/Blueprint/Weapon/WeaponBP.WeaponBP_C" (`self.GetTransform` self) "Undefined" "OverrideRootScale" null self))
  (bind _output_get (set `self.Weapon` _returnvalue))
  (`self.K2_AttachToComponent` _output_get (`self.Mesh`) "HandRSocket" "SnapToTarget" "SnapToTarget" "SnapToTarget" true))

(event `InputAxis|Move_Up`
  (params (AxisValue :type "Float (single-precision)"))
  ;[1 1 1] Movement
  (`self.AddMovementInput` (1.0 0.0 0.0) AxisValue))

(event `InputAxis|Move_Right`
  (params (AxisValue :type "Float (single-precision)"))
  ;[1 1 1] Movement
  (`self.AddMovementInput` (0.0 1.0 0.0) AxisValue))

(event `InputAxis|Look_Up`
  (params (AxisValue :type "Float (single-precision)"))
  ;[1 1 1] Look
  (`Controller.SetControlRotation` (`GameplayStatics.GetPlayerController` 0) (`KismetMathLibrary.Conv_VectorToRotator` (`KismetMathLibrary.MakeVector` AxisValue (stale `InputAxis|Look_Right` AxisValue)))))

(event `InputAxis|Look_Right`
  (params (AxisValue :type "Float (single-precision)"))
  ;[1 1 1] Look
)

(event `InputAction|FireWeapon`
  (params (Key :type "Key Structure"))
  (bind _weapon (`self.Weapon`))
  ;[1 1 1] Fire
  (:`Pressed`
    (`/Game/Blueprint/Weapon/WeaponBP.PullTrigger` _weapon))
  (:`Released`
    (`/Game/Blueprint/Weapon/WeaponBP.ReleaseTrigger` _weapon)))

(fn `UserConstructionScript`
  (`parent.UserConstructionScript`))